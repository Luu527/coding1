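; BP_Item is an item Blueprint with a name, an elemental type and damage, apparently a test of elemental damage logic.
; The construction script replaces the default "Item" name with a random month name from a small list.
; GetDamage doubles damage when the victim's element sits opposite in the four-value enum, using modulo arithmetic; an unused switch remains.
; BeginPlay calls an empty Constructor, then prints the name and damage against an Air victim.
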(event `self.ReceiveBeginPlay`
  (`self.Constructor`)
  (`KismetSystemLibrary.PrintString` (`KismetStringLibrary.Concat_StrStr` "Hey my name is " (`self.Name`)))
  (bind _damage (`self.GetDamage` "NewEnumerator3"))
  (`KismetSystemLibrary.PrintString` (`KismetStringLibrary.Concat_StrStr` "Elem type is  " (`|GetEnumeratorNameAsString` (`self.ElementalType`)) " , victim is Air, damage = " (`KismetStringLibrary.Conv_IntToString` _damage)) true true (struct :`R` 1.0 :`G` 0.084169 :`B` 0.150547 :`A` 1.0) 5.0))

(fn `Constructor`)

(fn `GetDamage`
  (params (VictimElementType :type "/Game/ElementalType Enum" :default "NewEnumerator1"))
  (returns (Damage :type Integer))
  (locals (ReturnedDamage :type Integer))
  (set `local.ReturnedDamage` (`self.Damage`))
  (if (== (mod (+ VictimElementType 2) 4) (`KismetMathLibrary.Conv_ByteToInt` (`self.ElementalType`)))
    (set `local.ReturnedDamage` (* (`self.Damage`) 2)))
  (return (`local.ReturnedDamage`)))

(fn `UserConstructionScript`
  (bind _array (`|MakeArray` "June" "July" "May" "April"))
  (if (`KismetStringLibrary.EqualEqual_StrStr` (`self.Name`) "Item")
    (`KismetArrayLibrary.Array_Shuffle` _array)
    (set `self.Name` (`|GetArrayItem` _array (`KismetMathLibrary.RandomIntegerInRange` 0 (- (`KismetArrayLibrary.Array_Length` _array) 1))))))