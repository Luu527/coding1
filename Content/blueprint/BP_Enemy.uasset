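; BP_Enemy is an enemy actor that dies when the third-person player character overlaps its capsule.
; On BeginPlay it fills an unset name and material by shuffling its candidate arrays, applies the material to its body and sphere, and prints debug messages.
; The player overlap drops Health below zero, and a looping Delay polls Health to destroy the actor instead of using Tick.
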(event `self.ReceiveBeginPlay`
  (bind _names (`self.Names`))
  (bind _material (`self.Material`))
  (`|ExecutionSequence`
    (:`then_0`
      ;[1 1 1] EVERY 0.2 seconds,  check to see if health <=0, if so, destory ourselves.
      (`KismetSystemLibrary.Delay` 0.2 :!label _label)
      (if (<= (`self.Health`) 0.0)
        (`self.K2_DestroyActor`)
        (else
          (goto _label))))
    (:`then_1`
      (if (== (`self.Enemy Name`) "None")
        (`KismetArrayLibrary.Array_Shuffle` _names)
        (bind _output_get (set `self.Enemy Name` (`|GetArrayItem` _names)))
        (`KismetSystemLibrary.PrintString` (`KismetStringLibrary.Concat_StrStr` (`KismetStringLibrary.Conv_NameToString` _output_get) " exist!") true true (struct :`R` 0.907986 :`G` 0.152579 :`B` 0.203803 :`A` 1.0) 20.0)))
    (:`then_2`
      (`/Engine/EditorBlueprintResources/StandardMacros.IsValid` (`self.EnemyMaterial`)
        (:`Is Valid`
          (`KismetSystemLibrary.PrintString` "has material?" true true (struct :`R` 1.0 :`G` 0.061484 :`B` 0.537855 :`A` 1.0) 10.0))
        (:`Is Not Valid`
          (`KismetSystemLibrary.PrintString` "Doesn't have material" true true (struct :`G` 0.66 :`B` 1.0 :`A` 1.0) 10.0)
          (`KismetArrayLibrary.Array_Shuffle` _material)
          (set `self.EnemyMaterial` (`|GetArrayItem` _material))))
      (`PrimitiveComponent.SetMaterial` (`self.body`) 0 (`self.EnemyMaterial`))
      (`PrimitiveComponent.SetMaterial` (`self.Sphere`) 0 (`self.EnemyMaterial`)))))

(event `self.Capsule.OnComponentBeginOverlap`
  (params (OverlappedComponent :type "PrimitiveComponent Object Reference") (OtherActor :type "Actor Object Reference") (OtherComp :type "PrimitiveComponent Object Reference") (OtherBodyIndex :type Integer) (bFromSweep :type Boolean) (SweepResult :type "HitResult Structure (by ref)"))
  (cast `/Game/ThirdPerson/Blueprints/BP_ThirdPersonCharacter` OtherActor) ; did the player hit us?
  (set `self.Health` -1.0))

(fn `UserConstructionScript`)