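; BP_EnemySpawner is a wave spawner that repopulates the level with BP_Enemy whenever none are left.
; On BeginPlay it gathers all BP_EnemySpawnLocation actors, prints their count, spawns a first wave and starts the enemy check.
; Each wave rolls an 80% chance per location to spawn an enemy at its transform.
; The check event re-calls itself after a short Delay, forming an endless polling loop that triggers new waves.
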(event `self.ReceiveBeginPlay`
  (bind _outactors (`GameplayStatics.GetAllActorsOfClass` "/Game/blueprint/BP_EnemySpawnLocation.BP_EnemySpawnLocation_C")) ; The blue "out Actors" is just like aray inC++
  (`KismetSystemLibrary.PrintString` (`KismetStringLibrary.Concat_StrStr` "There are" (`KismetStringLibrary.Conv_IntToString` (`KismetArrayLibrary.Array_Length` _outactors)) "spawners in the level.") true true (struct :`R` 1.0 :`G` 0.056468 :`B` 0.122843 :`A` 1.0) 20.0)
  (`self.Spawn Enemies`)
  (`self.Check enemy Count`))

(event `Spawn Enemies`
  (for _array_element (stale `self.ReceiveBeginPlay` _outactors)
    (if (< (`KismetMathLibrary.RandomFloat`) 0.8)
      (`|SpawnActorFromClass` "/Game/blueprint/BP_Enemy.BP_Enemy_C" (`self.GetTransform` _array_element) "Undefined" "MultiplyWithRoot" null null))))

(event `Check enemy Count`
  (bind _outactors (`GameplayStatics.GetAllActorsOfClass` "/Game/blueprint/BP_Enemy.BP_Enemy_C"))
  (if (not (> (`KismetArrayLibrary.Array_Length` _outactors) 0))
    (`self.Spawn Enemies`))
  (`KismetSystemLibrary.Delay` 2.0)
  (`self.Check enemy Count`) ; back to the event you just create, " Check Enemy Count"\nso it can loop forever.\nRemember to add "Check Enemy Count" after the "spawn enemies"  node up there,\nat the end of the function\nthen it can loop.
)

(fn `UserConstructionScript`)