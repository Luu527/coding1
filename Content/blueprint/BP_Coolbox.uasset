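; BP_Coolbox is an actor that endlessly spawns BP_Key actors above its Cube component.
; On BeginPlay it caches a spawn point 200 units above the cube and prints its name and both locations as debug text.
; A Delay wired back into SpawnActor forms the loop, with the interval set by the SpawnDelay variable and each key given a random scale.
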(event `self.ReceiveBeginPlay`
  (bind _returnvalue (`SceneComponent.K2_GetComponentLocation` (`self.Cube`)))
  (set `self.keyspwanlocation` (+ _returnvalue (0.0 0.0 200.0))) ; Here is to build a new code.\n\nReason: Every it runs, "Luu" asking the location of it, it kind of expensive.\nSo instead, Build a new variable. \n\n  Build a new variable:    At left side bar, in VARIABLE tab, click " + "\n                                              Name it Keyspawnlocation.\n                                            change the variable type to "Vector" (Transform also works, cuz its a location)\n\nHow this works:          At the begining, get the location, add 200z, then "set" this variable.\n                                      This means "keyspawn location = this", this called seting the variable's value.\n\n To change the code:  At " Event BeginPlay", drag, and search the variable's name (keyspawn location).\n                                      Then you get this "SET".\n                                       Then you can drag the whole cauculation(cube ref, get world location, add 200z) to the SET.               \n                                       Then you can replace those long mass yellow lines (connect from "add z" to those spawn nodesand ) with the variable.\n                                        Drag "keyspawnlocation" from left side, direct to the location pin (or the convert pin)\n                                        Or you can drag it anywhere and selet "Get" in the pop out tab, then connect it to the location pin.
  (`KismetSystemLibrary.PrintString` (`KismetStringLibrary.Concat_StrStr` (`KismetSystemLibrary.GetDisplayName` self) "  exist!") true true (struct :`R` 1.0 :`G` 0.524306 :`B` 0.981389 :`A` 1.0) 10.0) ; just like cout, cout the text "bp exist!"
  (`KismetSystemLibrary.PrintString` (`KismetStringLibrary.Conv_VectorToString` _returnvalue) true true (struct :`R` 0.093325 :`G` 0.758134 :`B` 1.0 :`A` 1.0) 10.0) ; cout the location
  (`KismetSystemLibrary.PrintString` (`KismetStringLibrary.Conv_VectorToString` (`self.keyspwanlocation`)) true true (struct :`R` 1.0 :`G` 0.842978 :`A` 1.0) 10.0) ; cout the loction with +200
  (`|SpawnActorFromClass` "/Game/blueprint/BP_Key.BP_Key_C" (`KismetMathLibrary.MakeTransform` (`self.keyspwanlocation`) (struct) (* 1.0 (`KismetMathLibrary.RandomFloatInRange` 0.1 2.0))) "Undefined" "MultiplyWithRoot" null null :!label _label) ; Another way to spawn the ball above\nright click "Spawn Transform", split struct pin\nat loction pin, also can be splited in to x,y,z (float)\ncan be also reconbianed\n\nThen drag the location yello pin to this lolcation pin
  (`KismetSystemLibrary.Delay` (`self.SpawnDelay`)) ; (Delay)make it a loop\nDuration adjust to 1
  (goto _label))

(fn `UserConstructionScript`)